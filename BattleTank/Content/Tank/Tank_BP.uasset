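; Player-controllable tank Blueprint that binds input to aiming, firing, movement and camera switching.
; BeginPlay hands barrel, turret and track references to the TankAiming and TankMovement components, then links the Healthbar widget to this tank.
; Look axes rotate a spring arm and azimuth gimbal, fire and drive inputs forward to those components, and switch camera toggles first- and third-person cameras.
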(event EventBeginPlay
  (Class|TankAimingComponent|Initialize (Variables|Default|GetTankAiming) (Variables|Default|GetBarrel) (Variables|Default|GetTurret))
  (Class|TankMovementComponent|Initialize (Variables|Default|GetTankMovement) (Variables|Default|GetTankTrackLeft) (Variables|Default|GetTankTrackRight))
  (bind _ashealthbar (Utilities|Casting|CastToHealthbar (UserInterface|GetUserWidgetObject (Variables|Default|GetWidget))))
  (Variables|/Game/UI/Healthbar.Healthbar_C|SetMyTank _ashealthbar self))

(event Input|ActionEvents|InputActionfire
  (params (Key :type Key%20Structure))
  ;[1 1 1] Balistics Input Aiming
  (:Pressed
    (Class|TankAimingComponent|Fire (Variables|Default|GetTankAiming))))

(event Input|ActionEvents|InputActionswitchcamera
  (params (Key :type Key%20Structure))
  ;[1 1 1] Camera Swapping
  (:Pressed
    (Components|Activation|ToggleActive (Variables|Default|Getfirst%20person))
    (Components|Activation|ToggleActive (Variables|Default|Getthird%20person))))

(event Input|AxisEvents|InputAxisAimAzimuth
  (params (AxisValue :type Float%20%28single-precision%29))
  ;[1 1 1] Balistics Input Aiming
  (Transformation|AddLocalRotation (Variables|Default|GetAzimuth%20Gimbal) (Math|Rotator|MakeRotator 0.0 0.0 (* AxisValue 1e+01)) false false))

(event Input|AxisEvents|InputAxismoveforward
  (params (AxisValue :type Float%20%28single-precision%29))
  ;[1 1 1] Movement Input Binding
  (Class|TankMovementComponent|IntendMoveForward (Variables|Default|GetTankMovement) AxisValue))

(event Input|AxisEvents|InputAxisturnright
  (params (AxisValue :type Float%20%28single-precision%29))
  ;[1 1 1] Movement Input Binding
  (Class|TankMovementComponent|IntendTurnRight (Variables|Default|GetTankMovement) AxisValue))

(event Input|AxisEvents|InputAxisAimElevation
  (params (AxisValue :type Float%20%28single-precision%29))
  ;[1 1 1] Balistics Input Aiming
  (Transformation|AddLocalRotation (Variables|Default|GetSpring%20Arm) (Math|Rotator|MakeRotator 0.0 (* AxisValue 1e+01) 0.0) false false))

(fn ConstructionScript)

(fn InitializeHealthbarWidget
  (bind _ashealthbar (Utilities|Casting|CastToHealthbar (UserInterface|GetUserWidgetObject (Variables|Default|GetWidget))))
  (Variables|/Game/UI/Healthbar.Healthbar_C|SetMyTank _ashealthbar 0))